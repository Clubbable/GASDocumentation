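; GA_ThrowBomb_BP is the hero's gameplay ability for aiming and throwing a picked-up projectile.
; Activation applies an aim effect, zooms the camera boom in and shows the HUD reticle until input release.
; On release with a projectile held, it commits, builds effect specs with SetByCaller damage and passes them to the launch.
; Ending hides the reticle, clears specs and aim effects, and restores the camera.
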(event Ability|EventActivateAbility
  (bind _asgdhero_character (Utilities|Casting|CastToGDHeroCharacter (Ability|GetAvatarActorfromActorInfo)))
  (Variables|Default|SetOwningHero _asgdhero_character)
  (bind _returnvalue (Ability|ApplyGameplayEffectToOwner "/Game/GASDocumentation/Characters/Shared/GameplayEffectTemplates/GE_StandardAimBomb.GE_StandardAimBomb_C" (Ability|GetAbilityLevel)))
  (Variables|Default|SetGEAimBomb _returnvalue)
  ;[1 1 1] Zoom in
  (Variables|/Script/Engine.SpringArmComponent|SetTargetArmLength (Variables|/Script/GASDocumentation.GDHeroCharacter|GetCameraBoom (Variables|Default|GetOwningHero)) 1e+02)
  (CallFunction|SetReticleVisibility "Visible" (Variables|Default|GetOwningHero))
  (Ability|Tasks|WaitInputRelease true ; When the player releases Right Mouse Button, end the ability
    (:OnRelease
      (if (Class|GDHeroCharacter|HasPickedupAnyProjectiles (Variables|Default|GetOwningHero))
        (Ability|CommitAbility)
        (for _array_element (Class|GDHeroCharacter|GetCurrentProjectileEffects (Variables|Default|GetOwningHero))
          (bind _returnvalue_2 (Ability|GameplayEffect|AssignTagSetbyCallerMagnitude (Ability|MakeOutgoingGameplayEffectSpec _array_element (Math|Conversions|ToFloat(Integer) (Ability|GetAbilityLevel))) "(TagName=\"Data.Damage\")" (Class|GDHeroCharacter|GetCurrentProjectileDamage (Variables|Default|GetOwningHero))))
          (Utilities|Array|Add (Variables|Default|GetEffectHandles) _returnvalue_2))
        (Class|GDHeroCharacter|LaunchPickedupProjectile (Variables|Default|GetOwningHero) (Variables|Default|GetEffectHandles))
        (Ability|EndAbility)
        (else
          (Ability|EndAbility))))))

(event Ability|EventOnEndAbility
  (params (bWasCancelled :type Boolean))
  (bind _owninghero (Variables|Default|GetOwningHero))
  (CallFunction|SetReticleVisibility "Hidden" (Variables|Default|GetOwningHero))
  (Utilities|Array|Clear (Variables|Default|GetEffectHandles))
  (bind _returnvalue (Ability|ApplyGameplayEffectToOwner "/Game/GASDocumentation/Characters/Shared/GameplayEffectTemplates/GE_StandardAimBombRemoval.GE_StandardAimBombRemoval_C" (Ability|GetAbilityLevel)))
  (Variables|Default|SetGEAimBombRemoval _returnvalue)
  (Ability|RemoveGameplayEffectFromOwnerWithHandle (Variables|Default|GetGEAimBomb))
  (Ability|RemoveGameplayEffectFromOwnerWithHandle (Variables|Default|GetGEAimBombRemoval))
  ;[1 1 1] Reset zoom
  (Variables|/Script/Engine.SpringArmComponent|SetTargetArmLength (Variables|/Script/GASDocumentation.GDHeroCharacter|GetCameraBoom _owninghero) (Variables|/Script/GASDocumentation.GDHeroCharacter|GetStartingCameraBoomArmLength _owninghero)))

(fn SetReticleVisibility
  (params (Visibility :type ESlateVisibility%20Enum :default "Visible") (HeroCharacter :type GD%20Hero%20Character%20Object%20Reference))
  (bind _asgdplayer_controller (Utilities|Casting|CastToGDPlayerController (Pawn|GetController HeroCharacter)))
  (bind _asui_hud (Utilities|Casting|CastToUI_HUD (Variables|/Script/GASDocumentation.GDPlayerController|GetUIHUDWidget _asgdplayer_controller)))
  (Default|ChangeReticleState _asui_hud Visibility))